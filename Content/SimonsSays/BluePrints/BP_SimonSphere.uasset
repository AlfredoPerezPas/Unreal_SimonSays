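; Colored target sphere for a Simon Says game that registers a press when shot by the player.
; On a hit from a FirstPersonProjectile, it destroys the projectile and calls SpherePressed with its ColorCode.
; The construction script uses ColorCode to index a color array and sets the mesh materials' ColorCode vector parameter, so each instance shows its assigned color.
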(event EventBeginPlay)

(event Collision|EventActorBeginOverlap
  (params (OtherActor :type Actor%20Object%20Reference)))

(event EventTick
  (params (DeltaSeconds :type Float%20%28single-precision%29)))

(event Collision|EventHit
  (params (MyComp :type Primitive%20Component%20Object%20Reference) (Other :type Actor%20Object%20Reference) (OtherComp :type Primitive%20Component%20Object%20Reference) (bSelfMoved :type Boolean) (HitLocation :type Vector :default "0, 0, 0") (HitNormal :type Vector :default "0, 0, 0") (NormalImpulse :type Vector :default "0, 0, 0") (Hit :type Hit%20Result%20Structure%20%28by%20ref%29))
  (Utilities|Casting|CastToFirstPersonProjectile Other)
  (Actor|DestroyActor Other)
  (Default|CallSpherePressed (Variables|Default|GetColorCode)))

(fn ConstructionScript
  (bind _colorcode (Variables|Default|GetColorCode))
  (bind _newvar_0 (Variables|Default|GetNewVar_0))
  (bind _returnvalue (Math|Conversions|ToInteger(Byte) _colorcode))
  (bind _output (Utilities|Array|Get(acopy) _newvar_0 _returnvalue))
  (bind (_b _g _r) (Math|Color|BreakColor _output))
  (Rendering|Material|SetVectorParameterValueonMaterials (Variables|Default|GetMesh) "ColorCode" (Math|Vector|MakeVector (Math|Conversions|ToFloat(Byte) _r) (Math|Conversions|ToFloat(Byte) _g) (Math|Conversions|ToFloat(Byte) _b))))