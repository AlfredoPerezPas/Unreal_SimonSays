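; BP_Door is a door for the Simon Says game that opens when the win event fires.
; On BeginPlay it binds OpenDoor to the win event of the SL_SimonLight actors in the level.
; OpenDoor plays a slowed timeline that sets the door mesh's relative location, with the MoveRight flag deciding whether the Y movement is mirrored.
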(event Custom|OpenDoor
  ;[1 1 1] Ejecuta la animación de apertura de la puerta
  (Components|Timeline|SetPlayRate (Variables|Default|GetDoor_Move) 0.2)
  (bind _door_movement (Timeline|Door_Move Play)
    (:Update
      (Transformation|SetRelativeLocation (Variables|Default|GetDoor) (Math|Vector|MakeVector (.x _door_movement) (* (Variables|Default|Getdirection) (.y _door_movement)) (.z _door_movement)) false false))))

(event EventBeginPlay
  (Utilities|FlowControl|Sequence
    (:then_0
      (if (not (Variables|Default|GetmoveRight))
        (Variables|Default|Setdirection -1)))
    (:then_1
      (bind _outactors (Actor|GetAllActorsOfClass "/Game/SimonsSays/BluePrints/SL_SimonLight.SL_SimonLight_C"))
      (EventDispatchers|BindEventtoWin _outactors (delegate Custom|OpenDoor)))))

(fn ConstructionScript)