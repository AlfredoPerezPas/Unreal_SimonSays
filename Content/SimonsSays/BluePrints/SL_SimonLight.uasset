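; Spotlight that runs a Simon Says game, generating a random color code at BeginPlay and showing it through its light color.
; A BP_Button press starts playback, and BP_SimonSphere selections are checked against the code, extending the shown sequence each round until CallWin.
; A wrong pick resets progress and turns the light red.
; Tick drives playback through a Delay that paces each color and returns the light to white when idle.
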(event Custom|SphereSelection
  (params (Color :type E_ColorCode%20Enum :default "NewEnumerator0"))
  ;[1 1 1] SphereSelection
  (if (not (Variables|Variables|GetActivateSecuence))
    (if (Utilities|Enum|Equal(Enum) Color (Utilities|Array|Get(acopy) (Variables|SimonConvination|GetColorCode) (Variables|Variables|GetActualColorSuccess)))
      ;;[0.2314 1 0.2677] Success
      (if (>= (Variables|Variables|GetActualColorSuccess) (Variables|Variables|GetLastColorSuccess))
        (if (<= (Utilities|Array|Length (Variables|SimonConvination|GetColorCode)) (+ (Variables|Variables|GetLastColorSuccess) 1))
          (Default|CallWin)
          (else
            (Utilities|FlowControl|Sequence
              (:then_0
                (Variables|Variables|SetActualColorSuccess 0))
              (:then_1
                (Variables|Variables|SetLastColorSuccess (+ (Variables|Variables|GetLastColorSuccess) 1)))
              (:then_2
                (Variables|Variables|SetActivateSecuence true)))))
        (else
          (Variables|Variables|SetActualColorSuccess (+ (Variables|Variables|GetActualColorSuccess) 1))))
      (else
        ;;[1 0.3177 0.3177] Wrong - ResetGame
        (Utilities|FlowControl|Sequence
          (:then_0
            (Variables|Variables|SetActualColorSuccess 0))
          (:then_1
            (Variables|Variables|SetLastColorSuccess 0))
          (:then_2
            (Variables|Variables|SetWrongColor true)))))))

(event Custom|ButtonPressed
  (Variables|Variables|SetLastColorSuccess 0)
  (Variables|Variables|SetActivateSecuence true))

(event Custom|Activate_Secuence
  ;[1 1 1] LoopColor
  (if (Variables|Variables|GetWrongColor)
    ;;[1 0.2292 0.2292] Wrong
    (Rendering|Components|Light|SetLightColor (Variables|Default|GetSpotLightComponent) "(R=0.432292,G=0.006552,B=0.000000,A=1.000000)" true)
    (Variables|Variables|SetWrongColor false)
    (else
      (Utilities|FlowControl|Delay (Variables|SimonConvination|GetTimeBetweenColors))
      (if (Variables|Variables|GetActivateSecuence)
        (Utilities|FlowControl|Sequence
          (:then_0
            ;;[0.8868 0.3476 1] SetActualColor
            (Rendering|Components|Light|SetLightColor (Variables|Default|GetSpotLightComponent) (Math|Conversions|ToLinearColor(Color) (Utilities|Array|Get(acopy) (Variables|Colors|GetColors) (Math|Conversions|ToInteger(Byte) (Utilities|Array|Get(acopy) (Variables|SimonConvination|GetColorCode) (Variables|Variables|GetActualColorShow))))) true))
          (:then_1
            (if (<= (Variables|Variables|GetLastColorSuccess) (Variables|Variables|GetActualColorShow))
              ;;[1 0.1771 0.1771] Stop
              (Utilities|FlowControl|Sequence
                (:then_0
                  (Variables|Variables|SetActivateSecuence false))
                (:then_1
                  (Variables|Variables|SetActualColorShow 0)))
              (else
                ;;[1 1 1] NextColor
                (Variables|Variables|SetActualColorShow (+ (Variables|Variables|GetActualColorShow) 1))))))
        (else
          ;;[1 0.8438 0] SetStandardColor
          (Rendering|Components|Light|SetLightColor (Variables|Default|GetSpotLightComponent) "(R=1.000000,G=1.000000,B=1.000000,A=1.000000)" true))))))

(event EventBeginPlay
  (bind _randomcodelength (Variables|SimonConvination|GetRandomCodeLength))
  (Utilities|FlowControl|Sequence
    (:then_0
      ;[1 1 1] RandomCode
      (Utilities|Array|Resize (Variables|SimonConvination|GetColorCode) _randomcodelength)
      (for _index (range 0 _randomcodelength)
        (Utilities|Array|SetArrayElem (Variables|SimonConvination|GetColorCode) _index (Utilities|Enum|ByteToEnumE_ColorCode (Math|Conversions|ToByte(Integer) (Math|Random|RandomIntegerinRange 0 (- (|GetNumEnumEntries) 1)))))))
    (:then_1
      (bind _outactors (Actor|GetAllActorsOfClass "/Game/SimonsSays/BluePrints/BP_Button.BP_Button_C"))
      (EventDispatchers|BindEventtoPressed _outactors (delegate Custom|ButtonPressed)))
    (:then_2
      (bind _outactors_2 (Actor|GetAllActorsOfClass "/Game/SimonsSays/BluePrints/BP_SimonSphere.BP_SimonSphere_C"))
      (EventDispatchers|BindEventtoSpherePressed _outactors_2 (delegate Custom|SphereSelection)))))

(event EventTick
  (params (DeltaSeconds :type Float%20%28single-precision%29))
  (CallFunction|ActivateSecuence))

(fn ConstructionScript)